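; Player component that manages a multiplayer character's weapons and relays their use over the network.
; It spawns weapons attached to the character, sorts them into main, second, melee, special and grenade slots, and tracks the current one.
; Weapon use runs a local pre-check and pre-confirmed action, then server validation, then a client confirmation, all delegated to the weapon.
; CurrentWeapon's RepNotify attaches it to the visible mesh's weapon socket on non-server machines.
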(event Custom|WeaponActionOnClient
  (params (Possibility :type Boolean) (WeaponActionInfo :type S%20Weapon%20Action%20Info%20Structure))
  ;[1 1 1 1 14] Client Weapon Action
  (Default|ConfirmedUseWeapon (Variables|Default|GetCurrentWeapon) Possibility WeaponActionInfo))

(event Custom|WeaponActionOnServer
  (params (WeaponActionInfo :type S%20Weapon%20Action%20Info%20Structure))
  ;[1 1 1 1 14] Server Weapon Action
  (bind (_possibility _weaponactioninfoout) (Default|ConfirmationOfPossibility (Variables|Default|GetCurrentWeapon) WeaponActionInfo))
  (CallFunction|WeaponActiononClient _possibility _weaponactioninfoout))

(event EventBeginPlay
  (Variables|Default|SetCharacter (.AsBP%20Multiplayer%20Character (Utilities|Casting|CastToBP_MultiplayerCharacter (Components|GetOwner)))))

(fn CreateWeapon
  (params (Class :type BP%20Weapon%20Class%20Reference))
  (bind _character (Variables|Default|GetCharacter))
  (bind _returnvalue (Game|SpawnActorfromClass Class (Math|Transform|MakeTransform "0, 0, 0" "0, 0, 0" "1,1,1") "AlwaysSpawn" (Pawn|GetController _character) _character))
  (bind _output_get (LocalVariables|SetL_Weapon _returnvalue))
  (switch Utilities|FlowControl|Switch|SwitchonE_WeaponType (Variables|/Game/Blueprints/Weapons/BP_Weapon.BP_Weapon_C|GetWeaponType _output_get)
    (:NewEnumerator0
      (Variables|Default|SetMainWeapon (LocalVariables|GetL_Weapon)))
    (:NewEnumerator1
      (Variables|Default|SetSecondWeapon (LocalVariables|GetL_Weapon)))
    (:NewEnumerator4
      (Variables|Default|SetMeleeWeapon (LocalVariables|GetL_Weapon)))
    (:NewEnumerator2
      (Utilities|Array|Add (Variables|Default|GetSpecials) (LocalVariables|GetL_Weapon)))
    (:NewEnumerator3
      (Utilities|Array|Add (Variables|Default|GetGrenages) (LocalVariables|GetL_Weapon))))
  (Transformation|AttachActorToActor (LocalVariables|GetL_Weapon) (Variables|Default|GetCharacter) "None" "SnapToTarget" "SnapToTarget" "KeepRelative" true)
  (return (LocalVariables|GetL_Weapon)))

(fn SelectWeapon
  (params (Weapon :type BP%20Weapon%20Object%20Reference))
  (Variables|Default|SetCurrentWeapon Weapon))

(fn OnRepCurrentWeapon
  (if (not (Networking|IsServer))
    (Transformation|AttachComponentToComponent (Variables|Default|GetCurrentWeapon) (Default|GetVisibleMesh (Variables|Default|GetCharacter)) "SKT_Weapon" "KeepRelative" "KeepRelative" "KeepRelative" true)))

(fn UseCurrentWeapon
  (bind _currentweapon (Variables|Default|GetCurrentWeapon))
  (bind _possibility (Default|PreConfirmationOfPossibility _currentweapon))
  (if _possibility
    (bind _weaponactioninfoout (Default|PreConfirmedUseWeapon _currentweapon (Utilities|Struct|MakeS_WeaponActionInfo (Variables|/Script/Engine.PlayerState|GetPlayerId (Variables|/Script/Engine.Pawn|GetPlayerState (Variables|Default|GetCharacter))) 0 0)))
    (CallFunction|WeaponActiononServer _weaponactioninfoout)))
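; BP_Weapon is a weapon Blueprint that gates use on ammo and a delay between uses, apparently as a base class.
; PreConfirmationOfPossibility passes only when unlocked and ammo remains.
; PreConfirmedUseWeapon spends ammo, sets a timer-released lock and returns action info with the instigator and weapon IDs.
; ConfirmationOfPossibility always approves, passing the info through, and ConfirmedUseWeapon is an empty hook for the confirmed action.
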(fn ConstructionScript)

(fn PreConfirmedUseWeapon
  (params (WeaponActionInfoIn :type S%20Weapon%20Action%20Info%20Structure))
  (Variables|Default|SetAmmo (Math|Float|Max(Float) (- (Variables|Default|GetAmmo) (Variables|Default|GetAmmoReductionFactor)) 0.0))
  (Utilities|Time|SetTimerbyFunctionName 0 "TurnOffLockByDelay" (Variables|Default|GetDelayToUse))
  (Variables|Default|SetLockedByDelay true)
  (return (Utilities|Struct|MakeS_WeaponActionInfo (.instigatorid WeaponActionInfoIn) (Variables|Default|GetWeaponId) 0)))

(fn TurnOffLockbyDelay
  (Variables|Default|SetLockedByDelay false))

(fn PreConfirmationOfPossibility
  (return (and (not (Variables|Default|GetLockedByDelay)) (> (Variables|Default|GetAmmo) 0.0))))

(fn ConfirmationOfPossibility
  (params (WeaponActionInfoIn :type S%20Weapon%20Action%20Info%20Structure))
  (return true WeaponActionInfoIn))

(fn ConfirmedUseWeapon
  (params (WeaponActionInfo :type S%20Weapon%20Action%20Info%20Structure)))
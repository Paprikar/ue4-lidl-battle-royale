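; Multiplayer hitscan rifle that extends a parent weapon class's use-and-confirm flow, currently with only debug feedback and no damage.
; PreConfirmedUseWeapon line-traces from the first-person camera along the owner's forward vector and records the hit character's PlayerId, or -1.
; Possibility checks defer to the parent.
; ConfirmedUseWeapon skips the locally controlled instigator; otherwise it resolves that ID to a character, prints the outcome and draws non-server debug traces.
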(event Custom|DEBUG_DrawTrace
  (params (Start :type Vector) (End :type Vector) (Hit :type Vector))
  (if (not (Networking|IsServer))
    (Rendering|Debug|DrawDebugLine Start End "(R=0.000000,G=0.000000,B=1.000000,A=1.000000)" 5.0 1.0)
    (Rendering|Debug|DrawDebugSphere Hit 1e+01 12 "(R=1.000000,G=0.000000,B=0.000000,A=1.000000)" 5.0 1.0)))

(event EventBeginPlay
  (|CallParentFunction))

(event EventTick
  (params (DeltaSeconds :type Float%20%28single-precision%29))
  (|CallParentFunction DeltaSeconds))

(event Collision|EventActorBeginOverlap
  (params (OtherActor :type Actor%20Object%20Reference))
  (|CallParentFunction OtherActor))

(event EventConfirmedUseWeapon
  (params (Possibility :type Boolean) (WeaponActionInfo :type S%20Weapon%20Action%20Info%20Structure))
  (bind (_instigatorid _subjectid _objectid) (Utilities|Struct|BreakS_WeaponActionInfo WeaponActionInfo))
  (bind _returnvalue (Game|GetInstigator))
  (bind _asbp_multiplayer_character (Utilities|Casting|CastToBP_MultiplayerCharacter _returnvalue))
  (bind _playerstate (Variables|/Script/Engine.Pawn|GetPlayerState _asbp_multiplayer_character))
  (bind _playerid (Variables|/Script/Engine.PlayerState|GetPlayerId _playerstate))
  (if (== _instigatorid _playerid)
    (if (not (Pawn|IsLocallyControlled _asbp_multiplayer_character))
      (Development|PrintString (Utilities|String|Append (Utilities|String|ToString(Integer) _instigatorid) " @ Server Instigator: " (Utilities|String|ToString(Integer) _playerid)) true true "(R=1.000000,G=0.953993,B=0.000000,A=1.000000)" 15.0)
      (if (== _objectid -1)
        (Development|PrintString "Failed use" true true "(R=1.000000,G=0.017903,B=0.000000,A=1.000000)" 5.0 :!label _label)
        (else
          (bind _outactors (Actor|GetAllActorswithTag "MultiplayerCharacter"))
          (bind _array_element (Utilities|Array|ForEachLoopwithBreak _outactors :!label _label_2)
            (:LoopBody
              (bind _asbp_multiplayer_character_2 (Utilities|Casting|CastToBP_MultiplayerCharacter _array_element))
              (if (== (Variables|/Script/Engine.PlayerState|GetPlayerId (Variables|/Script/Engine.Pawn|GetPlayerState _asbp_multiplayer_character_2)) _objectid)
                (Variables|Default|SetObjectCharacter _asbp_multiplayer_character_2)
                (goto _label_2 Break)))
            (:Completed
              (CallFunction|DEBUGDrawTrace (Transformation|GetActorLocation) (Transformation|GetActorLocation (Variables|Default|GetObjectCharacter)) (Transformation|GetActorLocation (Variables|Default|GetObjectCharacter)))
              (if Possibility
                (Development|PrintString "Successful use" true true "(R=0.000000,G=1.000000,B=0.016063,A=1.000000)" 5.0)
                (else
                  (goto _label)))))))
      (else
        (Development|PrintString "SkippedVisualOnInitiator")))
    (else
      (Development|PrintString "UseWeaponError"))))

(fn ConstructionScript
  (|CallParentFunction))

(fn GetFireTrace
  (bind _asbp_multiplayer_character (Utilities|Casting|CastToBP_MultiplayerCharacter (Game|GetInstigator))
    (:then
      (bind _outhit (Collision|LineTraceByChannel (Transformation|GetWorldLocation (Variables|/Game/Blueprints/Player/BP_MultiplayerCharacter.BP_MultiplayerCharacter_C|GetCamera_1P _asbp_multiplayer_character)) (+ (Transformation|GetWorldLocation (Variables|/Game/Blueprints/Player/BP_MultiplayerCharacter.BP_MultiplayerCharacter_C|GetCamera_1P _asbp_multiplayer_character)) (* (Transformation|GetActorForwardVector (Components|GetOwner)) 10000)) "TraceTypeQuery2" false (Utilities|Array|MakeArray self (Game|GetInstigator)) "None" false))
      (CallFunction|DEBUGDrawTrace (.TraceStart (Collision|BreakHitResult _outhit)) (.TraceEnd (Collision|BreakHitResult _outhit)) (.Location (Collision|BreakHitResult _outhit)))
      (return _outhit))
    (:CastFailed
      (return ""))))

(fn PreConfirmedUseWeapon
  (params (WeaponActionInfoIn :type S%20Weapon%20Action%20Info%20Structure))
  (bind _weaponactioninfoout (|CallParentFunction WeaponActionInfoIn))
  (bind _hit (CallFunction|GetFireTrace))
  (if (.bSuccess (Utilities|Casting|CastToBP_MultiplayerCharacter (.HitActor (Collision|BreakHitResult _hit))))
    (Development|PrintString (Utilities|String|Append "Object Id: " (Utilities|String|ToString(Integer) (Variables|/Script/Engine.PlayerState|GetPlayerId (Variables|/Script/Engine.Pawn|GetPlayerState (.AsBP%20Multiplayer%20Character (Utilities|Casting|CastToBP_MultiplayerCharacter (.HitActor (Collision|BreakHitResult _hit)))))))))
    (return (Utilities|Struct|MakeS_WeaponActionInfo (.instigatorid _weaponactioninfoout) (.subjectid _weaponactioninfoout) (Variables|/Script/Engine.PlayerState|GetPlayerId (Variables|/Script/Engine.Pawn|GetPlayerState (.AsBP%20Multiplayer%20Character (Utilities|Casting|CastToBP_MultiplayerCharacter (.HitActor (Collision|BreakHitResult _hit))))))))
    (else
      (return (Utilities|Struct|MakeS_WeaponActionInfo (.instigatorid _weaponactioninfoout) (.subjectid _weaponactioninfoout) -1)))))

(fn ConfirmationOfPossibility
  (params (WeaponActionInfoIn :type S%20Weapon%20Action%20Info%20Structure))
  (bind (_possibility _weaponactioninfoout) (|CallParentFunction WeaponActionInfoIn))
  (return _possibility (Utilities|Struct|MakeS_WeaponActionInfo (.instigatorid _weaponactioninfoout) (.subjectid _weaponactioninfoout) (.objectid _weaponactioninfoout))))

(fn PreConfirmationOfPossibility
  (bind _possibility (|CallParentFunction))
  (return _possibility))